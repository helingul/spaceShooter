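; BP_player is a player-controlled spaceship that moves along control-yaw axes and fires projectiles from two barrels.
; Holding fire while alive runs a Gate and Delay loop, with the interval scaled by a fire-rate multiplier and clamped.
; A flag selects alternating barrels via FlipFlop or simultaneous shots, passing a damage multiplier to each projectile.
; ForceFiringNow and StopFiringNow events let firing be forced or stopped and locked.
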(event Custom|ForceFiringNow
  (if (not (Variables|Fire|GethasLockedFiring))
    (if (Variables|Default|GetcanFire)
      (Utilities|FlowControl|Sequence
        (:then_0
          (goto _label Open))
        (:then_1
          (Utilities|FlowControl|Gate true :!label _label
            (:Exit
              (Utilities|FlowControl|Sequence
                (:then_0
                  _)
                (:then_1
                  (Utilities|FlowControl|Delay (Math|Float|Clamp(Float) (* (Variables|Fire|GetfireRate) (Variables|Fire|GetfireRateMultiplier)) 0.033) :!label _label_2)
                  (Variables|Default|SetcanFire true)
                  (goto _label)))))))
      (else
        (Utilities|FlowControl|Sequence
          (:then_0
            (goto _label Open))
          (:then_1
            (goto _label_2)))))
    (if (Variables|Default|GetflipFlopFiring)
      ;[1 1 1] if you have two barrels to shout out of, you can do different settings in there
      (Utilities|FlowControl|FlipFlop
        (:A
          (Game|SpawnActorfromClass (Variables|Default|GetprojectileParent) (Math|Transform|MakeTransform (Transformation|GetWorldLocation (Variables|Default|GetfirstBarrel)) "0,-90.000000, 0") "Undefined" 0 (Variables|Fire|GetdamageMultiplier) 2e+03 0)
          (Variables|Default|SetcanFire false))
        (:B
          (Game|SpawnActorfromClass (Variables|Default|GetprojectileParent) (Math|Transform|MakeTransform (Transformation|GetWorldLocation (Variables|Default|GetsecondBarrel)) "0,-90.000000, 0") "Undefined" 0 (Variables|Fire|GetdamageMultiplier) 2e+03 0)
          (Variables|Default|SetcanFire false)))
      (else
        (Game|SpawnActorfromClass (Variables|Default|GetprojectileParent) (Math|Transform|MakeTransform (Transformation|GetWorldLocation (Variables|Default|GetfirstBarrel)) "0,-90.000000, 0") "Undefined" 0 (Variables|Fire|GetdamageMultiplier) 2e+03 0)
        (Game|SpawnActorfromClass (Variables|Default|GetprojectileParent) (Math|Transform|MakeTransform (Transformation|GetWorldLocation (Variables|Default|GetsecondBarrel)) "0,-90.000000, 0") "Undefined" 0 (Variables|Fire|GetdamageMultiplier) 2e+03 0)
        (Variables|Default|SetcanFire false)))))

(event Custom|StopFiringNow
  (params (lockFiringInput :type Boolean))
  (if lockFiringInput
    (Variables|Fire|SethasLockedFiring true)
    (Utilities|FlowControl|Gate true) ; enters at Close
  ))

(event EventBeginPlay)

(event Collision|EventActorBeginOverlap
  (params (OtherActor :type Actor%20Object%20Reference)))

(event Input|ActionEvents|InputActionFireButton
  (params (Key :type Key%20Structure :default "None"))
  (:Pressed
    (if (Variables|Default|GetisAlive)
      (if (not (Variables|Fire|GethasLockedFiring))
        (if (Variables|Default|GetcanFire)
          (Utilities|FlowControl|Sequence
            (:then_0
              (goto _label Open))
            (:then_1
              (Utilities|FlowControl|Gate true :!label _label
                (:Exit
                  (Utilities|FlowControl|Sequence
                    (:then_0
                      _)
                    (:then_1
                      (Utilities|FlowControl|Delay (Math|Float|Clamp(Float) (* (Variables|Fire|GetfireRate) (Variables|Fire|GetfireRateMultiplier)) 0.033) :!label _label_2)
                      (Variables|Default|SetcanFire true)
                      (goto _label)))))))
          (else
            (Utilities|FlowControl|Sequence
              (:then_0
                (goto _label Open))
              (:then_1
                (goto _label_2)))))
        (if (Variables|Default|GetflipFlopFiring)
          ;[1 1 1] if you have two barrels to shout out of, you can do different settings in there
          (Utilities|FlowControl|FlipFlop
            (:A
              (Game|SpawnActorfromClass (Variables|Default|GetprojectileParent) (Math|Transform|MakeTransform (Transformation|GetWorldLocation (Variables|Default|GetfirstBarrel)) "0,-90.000000, 0") "Undefined" 0 (Variables|Fire|GetdamageMultiplier) 2e+03 0)
              (Variables|Default|SetcanFire false))
            (:B
              (Game|SpawnActorfromClass (Variables|Default|GetprojectileParent) (Math|Transform|MakeTransform (Transformation|GetWorldLocation (Variables|Default|GetsecondBarrel)) "0,-90.000000, 0") "Undefined" 0 (Variables|Fire|GetdamageMultiplier) 2e+03 0)
              (Variables|Default|SetcanFire false)))
          (else
            (Game|SpawnActorfromClass (Variables|Default|GetprojectileParent) (Math|Transform|MakeTransform (Transformation|GetWorldLocation (Variables|Default|GetfirstBarrel)) "0,-90.000000, 0") "Undefined" 0 (Variables|Fire|GetdamageMultiplier) 2e+03 0)
            (Game|SpawnActorfromClass (Variables|Default|GetprojectileParent) (Math|Transform|MakeTransform (Transformation|GetWorldLocation (Variables|Default|GetsecondBarrel)) "0,-90.000000, 0") "Undefined" 0 (Variables|Fire|GetdamageMultiplier) 2e+03 0)
            (Variables|Default|SetcanFire false))))))
  (:Released
    (if (not (Variables|Fire|GethasLockedFiring))
      (goto _label Close))))

(event Input|AxisEvents|InputAxisUp/Down
  (params (AxisValue :type Float%20%28single-precision%29))
  ;[1 1 1] Spaceship movement
  (Pawn|Input|AddMovementInput (Math|Vector|GetForwardVector (Math|Rotator|MakeRotator 0.0 0.0 (.Yaw (Math|Rotator|BreakRotator (Pawn|GetControlRotation :!class /Script/Engine.Pawn))))) AxisValue false))

(event Input|AxisEvents|InputAxisLeft/Right
  (params (AxisValue :type Float%20%28single-precision%29))
  ;[1 1 1] Spaceship movement
  (Pawn|Input|AddMovementInput (Math|Vector|GetRightVector (Math|Rotator|MakeRotator 0.0 0.0 (.Yaw (Math|Rotator|BreakRotator (Pawn|GetControlRotation :!class /Script/Engine.Pawn))))) AxisValue false))

(fn ConstructionScript)