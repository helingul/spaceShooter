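; Parent projectile Blueprint that damages enemies or the player on overlap, as set by its HarmEnemies and HarmPlayer flags.
; The construction script applies ProjectileSpeed to the movement component, and BeginPlay sets rotation by a look-at from location to the velocity vector.
; Sphere overlap branches on the first actor tag, subtracts multiplied damage from Health unless the player is invincible, runs the target's health check, and destroys the projectile.
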(event OnComponentBeginOverlap(Sphere)
  (params (OverlappedComponent :type Primitive%20Component%20Object%20Reference) (OtherActor :type Actor%20Object%20Reference) (OtherComp :type Primitive%20Component%20Object%20Reference) (OtherBodyIndex :type Integer) (bFromSweep :type Boolean) (SweepResult :type Hit%20Result%20Structure%20%28by%20ref%29))
  (bind _asbp_enemy_parent (Utilities|Casting|CastToBP_EnemyParent OtherActor))
  (bind _asbp_player (Utilities|Casting|CastToBP_player OtherActor))
  ;[1 1 1] enemy health
  (switch name (Utilities|Array|Get(acopy) (Variables|/Script/Engine.Actor|GetTags OtherActor))
    (:Enemy
      (if (Variables|Default|GetHarm_Enemies)
        (if (> (Variables|/Game/Blueprints/BP_EnemyParent.BP_EnemyParent_C|Gethealth _asbp_enemy_parent) 0.0)
          (Variables|/Game/Blueprints/BP_EnemyParent.BP_EnemyParent_C|Sethealth _asbp_enemy_parent (- (Variables|/Game/Blueprints/BP_EnemyParent.BP_EnemyParent_C|Gethealth _asbp_enemy_parent) (* (Variables|Default|Getdamage) (Variables|Default|GetdamageMultiplier))))
          (Default|HealthCheck _asbp_enemy_parent))
        (Actor|DestroyActor)))
    (:Player
      (if (Variables|Default|GetHarm_Player)
        (if (Variables|/Game/Blueprints/BP_player.BP_player_C|GetisAlive _asbp_player)
          (if (not (Variables|/Game/Blueprints/BP_player.BP_player_C|GetisInvincible _asbp_player))
            (Variables|/Game/Blueprints/BP_player.BP_player_C|Sethealth _asbp_player (- (Variables|/Game/Blueprints/BP_player.BP_player_C|Gethealth _asbp_player) (* (Variables|Default|GetdamageMultiplier) (Variables|Default|Getdamage))))
            (Default|HealtCheck _asbp_player))
          (Actor|DestroyActor))))))

(event EventBeginPlay
  (Transformation|SetActorRotation (Math|Rotator|FindLookatRotation (Transformation|GetActorLocation) (Transformation|GetVelocity))))

(fn ConstructionScript
  (bind _projectilemovement (Variables|Default|GetProjectileMovement))
  (bind _projectilespeed (Variables|Default|GetprojectileSpeed))
  (Variables|/Script/Engine.ProjectileMovementComponent|SetInitialSpeed _projectilemovement _projectilespeed)
  (Variables|/Script/Engine.ProjectileMovementComponent|SetMaxSpeed _projectilemovement _projectilespeed))